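; BP_Wolf is a movable wolf that leaves footprint trails and reacts to overlaps with its GroundRange component.
; GroundRange overlaps toggle an Out flag and the mesh height, while Tick passes that component to the game mode and nudges the mesh along world Y.
; FootprintEvent plays or stops a timeline based on movement input, offsetting the left and right trail components vertically in alternation.
; BeginPlay initializes temperature, state and foot rest positions.
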(event `self.ReceiveBeginPlay`
  (bind _returnvalue_location (`KismetMathLibrary.BreakTransform` (`SceneComponent.GetRelativeTransform` (`self.BP_TrailComponentFootR`))))
  (bind _returnvalue_location_2 (`KismetMathLibrary.BreakTransform` (`SceneComponent.GetRelativeTransform` (`self.BP_TrailComponentFootL`))))
  (set `self.Now Temperature` (`self.Max Temperature`))
  (set `self.State` "NewEnumerator0")
  (set `self.Lfoot` _returnvalue_location_2)
  (set `self.Rfoot` _returnvalue_location))

(event `self.ReceiveTick`
  (params (DeltaSeconds :type "Float (single-precision)"))
  (bind _mesh (`self.Mesh`))
  (message `/Game/MyContent/BP/System/BP_Interface.Collision Check` (`GameplayStatics.GetGameMode`) (`self.Ground Range`))
  (`SceneComponent.K2_SetWorldLocation` _mesh (+ (`SceneComponent.K2_GetComponentLocation` _mesh) (0.0 1.0 0.0)) false false))

(event `self.Ground Range.OnComponentBeginOverlap`
  (params (OverlappedComponent :type "PrimitiveComponent Object Reference") (OtherActor :type "Actor Object Reference") (OtherComp :type "PrimitiveComponent Object Reference") (OtherBodyIndex :type Integer) (bFromSweep :type Boolean) (SweepResult :type "HitResult Structure (by ref)"))
  (set `self.Out` true)
  (`SceneComponent.K2_SetRelativeLocation` (`self.Mesh`) (0.0 0.0 -40.0) false false))

(event `Footprint Event`
  (bind (_lfoot_x _lfoot_y _lfoot_z) (`KismetMathLibrary.BreakVector` (`self.Lfoot`)))
  (bind (_rfoot_x _rfoot_y _rfoot_z) (`KismetMathLibrary.BreakVector` (`self.Rfoot`)))
  ;[1 1 1] Footprint
  (if (and (== (`self.GetInputAxisValue`) 0.0) (== (`self.GetInputAxisValue`) 0.0))
    (bind (_direction `_新規track_0`) (`Timeline|FootprintL` :!via `Stop` :!label _label)
      (:`Update`
        (`SceneComponent.K2_SetRelativeLocation` (`self.BP_TrailComponentFootL`) (`KismetMathLibrary.MakeVector` _lfoot_x _lfoot_y (+ _lfoot_z (* `_新規track_0` 50.0))) true false)
        (`SceneComponent.K2_SetRelativeLocation` (`self.BP_TrailComponentFootR`) (`KismetMathLibrary.MakeVector` _rfoot_x _rfoot_y (+ _rfoot_z (* (- `_新規track_0` 1.0) -50.0))) true false)))
    (else
      (goto _label))))

(event `self.Ground Range.OnComponentEndOverlap`
  (params (OverlappedComponent :type "PrimitiveComponent Object Reference") (OtherActor :type "Actor Object Reference") (OtherComp :type "PrimitiveComponent Object Reference") (OtherBodyIndex :type Integer))
  (set `self.Out` false)
  (`SceneComponent.K2_SetRelativeLocation` (`self.Mesh`) (0.0 0.0 -90.0) false false))

(fn `UserConstructionScript`
  (`/Game/MyContent/TrailSystem/Blueprints/BP_TrailVisualizer.VisualizeTrailComponents`))