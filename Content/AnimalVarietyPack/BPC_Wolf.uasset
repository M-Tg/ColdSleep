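; Wolf character Blueprint that shifts its mesh vertically in response to overlaps on its GroundRange component.
; Each tick it passes GroundRange to the game mode's CollisionCheckMessage.
; Beginning an overlap sets the Out flag and raises the mesh, while ending one clears the flag and lowers it.
; The Walk function is an empty stub, and the only State assignment is unconnected.
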(event `self.ReceiveBeginPlay`)

(event `self.ReceiveTick`
  (params (DeltaSeconds :type "Float (single-precision)"))
  (message `/Game/MyContent/BP/System/BP_Interface.Collision Check` (`GameplayStatics.GetGameMode`) (`self.Ground Range`)))

(event `self.Ground Range.OnComponentBeginOverlap`
  (params (OverlappedComponent :type "PrimitiveComponent Object Reference") (OtherActor :type "Actor Object Reference") (OtherComp :type "PrimitiveComponent Object Reference") (OtherBodyIndex :type Integer) (bFromSweep :type Boolean) (SweepResult :type "HitResult Structure (by ref)"))
  (set `self.Out` true)
  (`SceneComponent.K2_SetRelativeLocation` (`self.Mesh`) (0.0 0.0 -40.0) false false))

(event `self.Ground Range.OnComponentEndOverlap`
  (params (OverlappedComponent :type "PrimitiveComponent Object Reference") (OtherActor :type "Actor Object Reference") (OtherComp :type "PrimitiveComponent Object Reference") (OtherBodyIndex :type Integer))
  (set `self.Out` false)
  (`SceneComponent.K2_SetRelativeLocation` (`self.Mesh`) (0.0 0.0 -90.0) false false))

(fn `UserConstructionScript`)

(fn `Walk`)