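; Dog character that moves by a state machine and spawns snow effects as footprints.
; Each Tick copies State to ABP_Dog, then walks to a target, turns, dashes, runs to the player or follows them.
; Walk and To Player switch to Idle within range, while Chase just stops.
; Snow spawns from hand trail components based on height; GroundCheck is never called, and OrderDog only prints a placeholder.
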(event `/Game/MyContent/BP/System/BP_Interface.Order Dog`
  (params (Val :type Boolean))
  (`KismetSystemLibrary.PrintString` "Hello"))

(event `self.ReceiveBeginPlay`)

(event `self.ReceiveTick`
  (params (DeltaSeconds :type "Float (single-precision)"))
  (bind _returnvalue (`self.K2_GetActorLocation`))
  (bind _returnvalue_2 (`self.GetActorForwardVector`))
  (bind _returnvalue_3 (`self.K2_GetActorLocation`))
  (bind _returnvalue_4 (`self.K2_GetActorLocation`))
  (bind (_nowtarget_x _nowtarget_y) (`KismetMathLibrary.BreakVector` (`self.NowTarget`)))
  (`self.Foot Print`)
  (bind _output_get (set `/Game/AnimalVarietyPack/ABP_Dog.AnimState` (`self.State`) (cast `/Game/AnimalVarietyPack/ABP_Dog` (`SkeletalMeshComponent.GetAnimInstance` (`self.Mesh`)) :!pure true)))
  (switch `/Game/AnimalVarietyPack/BP_WolfStateEnum` _output_get
    (:`NewEnumerator2`
      ;[1 1 1] 方向転換
      (bind _output_get_2 (set `self.NowTarget` (`KismetMathLibrary.MakeVector` (.x (`self.TargetLocation`)) (.y (`self.TargetLocation`)) (.z _returnvalue_3))))
      (`self.K2_SetActorRotation` (`KismetMathLibrary.RInterpTo` (`KismetMathLibrary.FindLookAtRotation` _returnvalue_3 _output_get_2) (struct) (`GameplayStatics.GetWorldDeltaSeconds`) 1.0))
      (`self.AddMovementInput` (`self.GetActorForwardVector`) (`self.Walk Speed`))
      (`self.Reach Target`))
    (:`NewEnumerator4`
      (`SceneComponent.K2_AddLocalRotation` (`self.CapsuleComponent`) (struct :`Yaw` -4.0) false false)
      (`self.AddMovementInput` (`self.GetActorForwardVector`) (`self.Walk Speed`)))
    (:`NewEnumerator7`
      (`self.AddMovementInput` (`self.GetActorForwardVector`) (`self.Run Speed`)))
    (:`NewEnumerator10`
      (bind _output_get_3 (set `self.NowTarget` (`KismetMathLibrary.MakeVector` (.x (`SceneComponent.K2_GetComponentLocation` (`Character.CapsuleComponent` (`GameplayStatics.GetPlayerCharacter` 0)))) (.y (`SceneComponent.K2_GetComponentLocation` (`Character.CapsuleComponent` (`GameplayStatics.GetPlayerCharacter` 0)))) (.z _returnvalue_4))))
      (`self.K2_SetActorRotation` (`KismetMathLibrary.RInterpTo` (`KismetMathLibrary.FindLookAtRotation` _returnvalue_4 _output_get_3) (struct) (`GameplayStatics.GetWorldDeltaSeconds`) 1.0))
      (`self.AddMovementInput` (`self.GetActorForwardVector`) (`self.Run Speed`))
      (`self.Reach Target`))
    (:`NewEnumerator11`
      (bind _output_get_4 (set `self.NowTarget` (`KismetMathLibrary.MakeVector` (.x (`SceneComponent.K2_GetComponentLocation` (`Character.CapsuleComponent` (`GameplayStatics.GetPlayerCharacter` 0)))) (.y (`SceneComponent.K2_GetComponentLocation` (`Character.CapsuleComponent` (`GameplayStatics.GetPlayerCharacter` 0)))) (.z _returnvalue))))
      (`self.K2_SetActorRotation` (`KismetMathLibrary.RInterpTo` (`KismetMathLibrary.FindLookAtRotation` _returnvalue _output_get_4) (struct) (`GameplayStatics.GetWorldDeltaSeconds`) 1.0))
      (if (and (< (`KismetMathLibrary.Abs` (- (.x (`self.K2_GetActorLocation`)) _nowtarget_x)) 100.0) (< (`KismetMathLibrary.Abs` (- (.y (`self.K2_GetActorLocation`)) _nowtarget_y)) 100.0))
        (`self.AddMovementInput` _returnvalue_2 0.0)
        (else
          (`self.AddMovementInput` _returnvalue_2 (`self.Walk Speed`)))))))

(event `self.GroundRange.OnComponentBeginOverlap`
  (params (OverlappedComponent :type "PrimitiveComponent Object Reference") (OtherActor :type "Actor Object Reference") (OtherComp :type "PrimitiveComponent Object Reference") (OtherBodyIndex :type Integer) (bFromSweep :type Boolean) (SweepResult :type "HitResult Structure (by ref)"))
  (cast `/Game/MyContent/BP/BPObject/BP_NosnowRange` OtherActor)
  (set `self.NoSnow` true))

(event `Reach Target`
  (bind (_nowtarget_x _nowtarget_y) (`KismetMathLibrary.BreakVector` (`self.NowTarget`)))
  (if (and (< (`KismetMathLibrary.Abs` (- (.x (`self.K2_GetActorLocation`)) _nowtarget_x)) 100.0) (< (`KismetMathLibrary.Abs` (- (.y (`self.K2_GetActorLocation`)) _nowtarget_y)) 100.0))
    (set `self.State` "NewEnumerator0")))

(event `self.GroundRange.OnComponentEndOverlap`
  (params (OverlappedComponent :type "PrimitiveComponent Object Reference") (OtherActor :type "Actor Object Reference") (OtherComp :type "PrimitiveComponent Object Reference") (OtherBodyIndex :type Integer)))

(event `Foot Print`
  (bind _bp_trailcomponenthandr (`self.BP_TrailComponentHandR`))
  (bind _bp_trailcomponenthandl (`self.BP_TrailComponentHandL`))
  (bind _z (.z (`self.K2_GetActorLocation`)))
  (if (>= (.z (`SceneComponent.K2_GetComponentLocation` _bp_trailcomponenthandr)) _z)
    (`|SpawnActorFromClass` "/Game/WorkSpace/koto/snow/MyContents/niagaraTest/snoweffect.snoweffect_C" (`KismetMathLibrary.MakeTransform` (.location (`SceneComponent.K2_GetComponentToWorld` _bp_trailcomponenthandr)) (* (.rotation (`SceneComponent.K2_GetComponentToWorld` _bp_trailcomponenthandr)) 90.0) (* (.scale (`SceneComponent.K2_GetComponentToWorld` _bp_trailcomponenthandr)) (2.0 2.0 0.001))) "Undefined" "OverrideRootScale" null null)
    (elif (>= (.z (`SceneComponent.K2_GetComponentLocation` _bp_trailcomponenthandl)) _z)
      (`|SpawnActorFromClass` "/Game/WorkSpace/koto/snow/MyContents/niagaraTest/snoweffect.snoweffect_C" (`KismetMathLibrary.MakeTransform` (.location (`SceneComponent.K2_GetComponentToWorld` _bp_trailcomponenthandl)) (.rotation (`SceneComponent.K2_GetComponentToWorld` _bp_trailcomponenthandl)) (* (.scale (`SceneComponent.K2_GetComponentToWorld` _bp_trailcomponenthandl)) (2.0 2.0 0.01))) "Undefined" "OverrideRootScale" null null))))

(fn `Ground Check`
  (bind _mesh (`self.Mesh`))
  (set `self.NoSnow` false)
  (message `/Game/MyContent/BP/System/BP_Interface.Collision Check` (`GameplayStatics.GetGameMode`) (`self.GroundRange`))
  (if true
    (`SceneComponent.K2_SetRelativeLocation` _mesh (0.0 0.0 -90.0) true false)
    (else
      (`SceneComponent.K2_SetRelativeLocation` _mesh (0.0 0.0 -40.0) true false))))

(fn `UserConstructionScript`
  (`/Game/MyContent/TrailSystem/Blueprints/BP_TrailVisualizer.VisualizeTrailComponents`))