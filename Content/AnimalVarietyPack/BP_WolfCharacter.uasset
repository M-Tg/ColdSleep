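; Wolf character that walks itself through the world, driving two trail components as left and right feet for footprints.
; Each tick it shifts Core along world X, or along Y while FrontBox overlaps, and passes both collision volumes to the GameMode.
; A timeline offsets the feet vertically in opposing phase.
; GroundRange overlaps adjust height and disable gravity on entry, while FallCheck lifts Core back up after a deep fall.
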(event `self.ReceiveBeginPlay`
  (bind _returnvalue_location (`KismetMathLibrary.BreakTransform` (`SceneComponent.GetRelativeTransform` (`self.BP_TrailComponentFootR`))))
  (bind _returnvalue_location_2 (`KismetMathLibrary.BreakTransform` (`SceneComponent.GetRelativeTransform` (`self.BP_TrailComponentFootL`))))
  (set `self.Lfoot` _returnvalue_location_2)
  (set `self.Rfoot` _returnvalue_location))

(event `self.ReceiveTick`
  (params (DeltaSeconds :type "Float (single-precision)"))
  (bind _core (`self.core`))
  (bind _core_2 (`self.core`))
  (`self.FallCheck`)
  (message `/Game/MyContent/BP/System/BP_Interface.Collision Check` (`GameplayStatics.GetGameMode`) (`self.Ground Range`))
  (message `/Game/MyContent/BP/System/BP_Interface.Collision Check` (`GameplayStatics.GetGameMode`) (`self.FrontBox`))
  (if (not (`self.TurnL`))
    (`SceneComponent.K2_SetWorldLocation` _core (+ (`SceneComponent.K2_GetComponentLocation` _core) (4.0 0.0 0.0)) false false)
    (`self.Footprint Event`)
    (else
      (`SceneComponent.K2_SetWorldLocation` _core_2 (+ (`SceneComponent.K2_GetComponentLocation` _core_2) (0.0 10.0 0.0)) false false)
      (`self.Footprint Event`))))

(event `self.Ground Range.OnComponentBeginOverlap`
  (params (OverlappedComponent :type "PrimitiveComponent Object Reference") (OtherActor :type "Actor Object Reference") (OtherComp :type "PrimitiveComponent Object Reference") (OtherBodyIndex :type Integer) (bFromSweep :type Boolean) (SweepResult :type "HitResult Structure (by ref)"))
  (bind _defaultsceneroot (`self.DefaultSceneRoot`))
  (set `self.Out` true)
  (`SceneComponent.K2_SetRelativeLocation` (`self.core`) (0.0 0.0 -20.0) false false)
  (`SceneComponent.K2_SetWorldLocation` _defaultsceneroot (+ (`SceneComponent.K2_GetComponentLocation` _defaultsceneroot) (0.0 0.0 50.0)) false false)
  (`PrimitiveComponent.SetEnableGravity` (`self.core`) false))

(event `Footprint Event`
  (bind (_lfoot_x _lfoot_y _lfoot_z) (`KismetMathLibrary.BreakVector` (`self.Lfoot`)))
  (bind (_rfoot_x _rfoot_y _rfoot_z) (`KismetMathLibrary.BreakVector` (`self.Rfoot`)))
  ;[1 1 1] Footprint
  (bind (_direction `_新規track_2`) (`Timeline|タイムライン_0`)
    (:`Update`
      (`SceneComponent.K2_SetRelativeLocation` (`self.BP_TrailComponentFootL`) (`KismetMathLibrary.MakeVector` _lfoot_x _lfoot_y (+ _lfoot_z (* `_新規track_2` 1000.0))) true false)
      (`SceneComponent.K2_SetRelativeLocation` (`self.BP_TrailComponentFootR`) (`KismetMathLibrary.MakeVector` _rfoot_x _rfoot_y (+ _rfoot_z (* (- `_新規track_2` 1.0) 1000.0))) true false))))

(event `self.Ground Range.OnComponentEndOverlap`
  (params (OverlappedComponent :type "PrimitiveComponent Object Reference") (OtherActor :type "Actor Object Reference") (OtherComp :type "PrimitiveComponent Object Reference") (OtherBodyIndex :type Integer))
  (set `self.Out` false)
  (`SceneComponent.K2_SetRelativeLocation` (`self.core`) (0.0 0.0 -90.0) false false))

(event `self.FrontBox.OnComponentBeginOverlap`
  (params (OverlappedComponent :type "PrimitiveComponent Object Reference") (OtherActor :type "Actor Object Reference") (OtherComp :type "PrimitiveComponent Object Reference") (OtherBodyIndex :type Integer) (bFromSweep :type Boolean) (SweepResult :type "HitResult Structure (by ref)"))
  (set `self.TurnL` true))

(event `self.FrontBox.OnComponentEndOverlap`
  (params (OverlappedComponent :type "PrimitiveComponent Object Reference") (OtherActor :type "Actor Object Reference") (OtherComp :type "PrimitiveComponent Object Reference") (OtherBodyIndex :type Integer))
  (set `self.TurnL` false))

(fn `FallCheck`
  (bind _core (`self.core`))
  (bind _returnvalue (`SceneComponent.K2_GetComponentLocation` _core))
  (if (< (.z _returnvalue) -2000.0)
    (`SceneComponent.K2_SetWorldLocation` _core (+ _returnvalue (0.0 0.0 6000.0)) false false)))

(fn `UserConstructionScript`
  (`/Game/MyContent/TrailSystem/Blueprints/BP_TrailVisualizer.VisualizeTrailComponents`))