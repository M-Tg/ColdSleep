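; Dog animation actor in the Sequencer folder that spawns snow footprint effects from its hand trail components.
; Each tick, FootPrint spawns Snoweffect 50 units below the right hand component if it is at or above the actor's origin, otherwise tests the left.
; GroundRange overlap with BP_NosnowRange sets NoSnow, which FootPrint ignores.
; GroundCheck, which adjusts mesh height, is never run.
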(event `self.ReceiveBeginPlay`
  (set `self.State` "NewEnumerator2"))

(event `self.ReceiveTick`
  (params (DeltaSeconds :type "Float (single-precision)"))
  (`self.Foot Print`))

(event `self.GroundRange.OnComponentBeginOverlap`
  (params (OverlappedComponent :type "PrimitiveComponent Object Reference") (OtherActor :type "Actor Object Reference") (OtherComp :type "PrimitiveComponent Object Reference") (OtherBodyIndex :type Integer) (bFromSweep :type Boolean) (SweepResult :type "HitResult Structure (by ref)"))
  (cast `/Game/MyContent/BP/BPObject/BP_NosnowRange` OtherActor)
  (set `self.NoSnow` true))

(event `self.GroundRange.OnComponentEndOverlap`
  (params (OverlappedComponent :type "PrimitiveComponent Object Reference") (OtherActor :type "Actor Object Reference") (OtherComp :type "PrimitiveComponent Object Reference") (OtherBodyIndex :type Integer)))

(event `Foot Print`
  (bind _bp_trailcomponenthandr (`self.BP_TrailComponentHandR`))
  (bind _bp_trailcomponenthandl (`self.BP_TrailComponentHandL`))
  (bind _z (.z (`self.K2_GetActorLocation`)))
  (if (>= (.z (`SceneComponent.K2_GetComponentLocation` _bp_trailcomponenthandr)) _z)
    (`|SpawnActorFromClass` "/Game/WorkSpace/koto/snow/MyContents/niagaraTest/snoweffect.snoweffect_C" (`KismetMathLibrary.MakeTransform` (+ (.location (`SceneComponent.K2_GetComponentToWorld` _bp_trailcomponenthandr)) (0.0 0.0 -50.0)) (.rotation (`SceneComponent.K2_GetComponentToWorld` _bp_trailcomponenthandr)) (.scale (`SceneComponent.K2_GetComponentToWorld` _bp_trailcomponenthandr))) "Undefined" "OverrideRootScale" null null)
    (elif (>= (.z (`SceneComponent.K2_GetComponentLocation` _bp_trailcomponenthandl)) _z)
      (`|SpawnActorFromClass` "/Game/WorkSpace/koto/snow/MyContents/niagaraTest/snoweffect.snoweffect_C" (`KismetMathLibrary.MakeTransform` (+ (.location (`SceneComponent.K2_GetComponentToWorld` _bp_trailcomponenthandl)) (0.0 0.0 -50.0)) (.rotation (`SceneComponent.K2_GetComponentToWorld` _bp_trailcomponenthandl)) (.scale (`SceneComponent.K2_GetComponentToWorld` _bp_trailcomponenthandl))) "Undefined" "OverrideRootScale" null null))))

(fn `Ground Check`
  (bind _mesh (`self.Mesh`))
  (set `self.NoSnow` false)
  (message `/Game/MyContent/BP/System/BP_Interface.Collision Check` (`GameplayStatics.GetGameMode`) (`self.GroundRange`))
  (if true
    (`SceneComponent.K2_SetRelativeLocation` _mesh (0.0 0.0 -90.0) true false)
    (else
      (`SceneComponent.K2_SetRelativeLocation` _mesh (0.0 0.0 -40.0) true false))))

(fn `UserConstructionScript`
  (`/Game/MyContent/TrailSystem/Blueprints/BP_TrailVisualizer.VisualizeTrailComponents`))