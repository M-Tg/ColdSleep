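; Bonfire object that shows a fire particle effect when the game instance's LevelOfFire is above zero at BeginPlay.
; The construction script applies a configurable mesh and scale.
; When lit, it uses the Lv1 template with configurable offset, scale and smoke/distortion emitter toggles; otherwise it clears the template.
; A disconnected switch would pick Lv1–Lv3 templates by fire level, but never runs, so Lv2 and Lv3 are unused.
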(event `self.ReceiveBeginPlay`
  (bind _particlesystem (`self.Particlesystem`))
  (if (<= (`/Game/MyContent/BP/System/BP_GameInstance.LevelOfFire` (cast `/Game/MyContent/BP/System/BP_GameInstance` (`GameplayStatics.GetGameInstance`) :!pure true)) 0)
    (`ParticleSystemComponent.SetTemplate` _particlesystem null)
    (else
      (`ParticleSystemComponent.SetTemplate` _particlesystem (`self.Lv1Fire`))
      (`SceneComponent.K2_SetRelativeLocation` _particlesystem (`self.Particle_offset`) false false)
      (`SceneComponent.SetRelativeScale3D` _particlesystem (`self.Particle_Scale`))
      (`ParticleSystemComponent.SetEmitterEnable` (`self.ParticleSystem`) "smoke" (`self.Smoke_Emitter_Enable`))
      (`ParticleSystemComponent.SetEmitterEnable` (`self.ParticleSystem`) "Distortion" (`self.Distortion_Emittter_Enable`)))))

(event `self.ReceiveTick`
  (params (DeltaSeconds :type "Float (single-precision)")))

(fn `UserConstructionScript`
  (bind _staticmeshcomponent (`self.StaticMeshComponent`))
  (`StaticMeshComponent.SetStaticMesh` _staticmeshcomponent (`self.Staticmesh`))
  (`SceneComponent.SetRelativeScale3D` _staticmeshcomponent (`self.Scale`)))