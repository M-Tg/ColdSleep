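; Weather actor that controls snowfall particle effects around the player and the house.
; Each tick it moves the overhead snow emitter above the player's capsule and hides it while the player's Covered flag is set.
; The game mode's InHouse flag then swaps between the outdoor snow emitters and a separate house snow emitter, which is placed at a fixed world position.
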(event `self.ReceiveTick`
  (params (DeltaSeconds :type "Float (single-precision)"))
  (bind _ps_housesnow (`self.PS_HouseSnow`))
  (`SceneComponent.K2_SetWorldLocation` (`self.PS_AboveSnow`) (+ (`SceneComponent.K2_GetComponentLocation` (`Character.CapsuleComponent` (`GameplayStatics.GetPlayerCharacter` 0))) (0.0 0.0 500.0)) false false)
  (if (`/Game/FirstPersonBP/Blueprints/BP_PlayerVer4.Covered` (cast `/Game/FirstPersonBP/Blueprints/BP_PlayerVer4` (`GameplayStatics.GetPlayerCharacter` 0) :!pure true))
    (`SceneComponent.SetHiddenInGame` (`self.PS_AboveSnow`) true false)
    (else
      (`SceneComponent.SetHiddenInGame` (`self.PS_AboveSnow`) false false)))
  (if (`/Game/MyContent/BP/System/BP_GameMode.InHouse` (cast `/Game/MyContent/BP/System/BP_GameMode` (`GameplayStatics.GetGameMode`) :!pure true))
    (`SceneComponent.SetHiddenInGame` (`self.PS_AboveSnow`) true false)
    (`SceneComponent.SetHiddenInGame` (`self.PS_Snow`) true false)
    (`SceneComponent.SetHiddenInGame` (`self.PS_Snow1`) true false)
    (`SceneComponent.SetHiddenInGame` (`self.PS_Snow2`) true false)
    (`SceneComponent.SetHiddenInGame` (`self.PS_Snow3`) true false)
    (`SceneComponent.SetHiddenInGame` (`self.PS_AboveSnow1`) true false)
    (`SceneComponent.SetHiddenInGame` (`self.PS_AboveSnow2`) true false)
    (`SceneComponent.SetHiddenInGame` (`self.PS_AboveSnow3`) true false)
    (`SceneComponent.SetHiddenInGame` (`self.PS_AboveSnow4`) true false)
    (`SceneComponent.SetHiddenInGame` _ps_housesnow false false)
    (`SceneComponent.K2_SetWorldLocation` _ps_housesnow (3000.0 1800.0 800.0) false false)
    (else
      (`SceneComponent.SetHiddenInGame` (`self.PS_Snow`) false false)
      (`SceneComponent.SetHiddenInGame` (`self.PS_Snow1`) false false)
      (`SceneComponent.SetHiddenInGame` (`self.PS_Snow2`) false false)
      (`SceneComponent.SetHiddenInGame` (`self.PS_Snow3`) false false)
      (`SceneComponent.SetHiddenInGame` (`self.PS_AboveSnow1`) false false)
      (`SceneComponent.SetHiddenInGame` (`self.PS_AboveSnow2`) false false)
      (`SceneComponent.SetHiddenInGame` (`self.PS_AboveSnow3`) false false)
      (`SceneComponent.SetHiddenInGame` (`self.PS_AboveSnow4`) false false)
      (`SceneComponent.SetHiddenInGame` _ps_housesnow true false))))

(fn `UserConstructionScript`)