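; BP_RandomWoodL is an actor that randomly scatters copies of a configurable actor class, presumably trees going by its name, around itself.
; On BeginPlay it loops up to LastIndex, adding child actor components at random X/Y offsets within a large square at zero relative height, then assigns InClass to each.
; The Construction Script holds a disconnected copy of the same loop, so scattering happens only at runtime.
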(event `self.ReceiveBeginPlay`
  (for _ (range (+ (`self.Last Index`) 1))
    (bind _returnvalue (`AddComponent|NODE_AddChildActorComponent-1` :`RelativeTransform` (`KismetMathLibrary.Conv_VectorToTransform` (`KismetMathLibrary.MakeVector` (`KismetMathLibrary.RandomFloatInRange` -4000.0 4000.0) (`KismetMathLibrary.RandomFloatInRange` -4000.0 4000.0) (`KismetMathLibrary.RandomFloatInRange` 0.0)))))
    (`ChildActorComponent.SetChildActorClass` _returnvalue (`self.In Class`))))

(fn `UserConstructionScript`)