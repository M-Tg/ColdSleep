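; BP_AppleSpawn is a spawner actor that places OI_Apple actors in the level at BeginPlay.
; It adds one child actor component for each transform in its AppleLocation array, up to LastIndex.
; It then gathers every OI_Apple in the world into AppleList and passes each its array index through SetIndex.
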(event `self.ReceiveBeginPlay`
  (for _index (range (+ (`self.Last Index`) 1))
    (bind _returnvalue (`AddComponent|NODE_AddChildActorComponent-3` :`RelativeTransform` (`|GetArrayItem` (`self.Apple Location`) _index)))
    (`ChildActorComponent.SetChildActorClass` _returnvalue "/Game/MyContent/BP/Object/OI_Apple.OI_Apple_C"))
  (bind _outactors (`GameplayStatics.GetAllActorsOfClass` "/Game/MyContent/BP/Object/OI_Apple.OI_Apple_C"))
  (bind _output_get (set `self.Apple List` _outactors))
  (for (_array_element _array_index) _output_get
    (`/Game/MyContent/BP/Object/OI_Apple.Set Index` _array_element _array_index)))

(fn `UserConstructionScript`)