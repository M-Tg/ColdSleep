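; Dog AI character that feeds Blackboard keys, presumably for a behavior tree steering the dog.
; Tick writes a BP_TargetDog as target, though its "closest" search compares dog-to-player distance, and flags player-to-target range, the last actor winning.
; OrderDog sets the order key.
; The older AnimState-driven movement and snow GroundCheck are disconnected; only the NoSnow overlap setter remains live.
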(event `self.ReceiveBeginPlay`)

(event `self.GroundRange.OnComponentBeginOverlap`
  (params (OverlappedComponent :type "PrimitiveComponent Object Reference") (OtherActor :type "Actor Object Reference") (OtherComp :type "PrimitiveComponent Object Reference") (OtherBodyIndex :type Integer) (bFromSweep :type Boolean) (SweepResult :type "HitResult Structure (by ref)"))
  (cast `/Game/MyContent/BP/BPObject/BP_NosnowRange` OtherActor)
  (set `self.NoSnow` true))

(event `self.GroundRange.OnComponentEndOverlap`
  (params (OverlappedComponent :type "PrimitiveComponent Object Reference") (OtherActor :type "Actor Object Reference") (OtherComp :type "PrimitiveComponent Object Reference") (OtherBodyIndex :type Integer)))

(event `Reach Target`
  (bind (_nowtarget_x _nowtarget_y) (`KismetMathLibrary.BreakVector` (`self.NowTarget`)))
  (if (and (< (`KismetMathLibrary.Abs` (- (.x (`self.K2_GetActorLocation`)) _nowtarget_x)) 100.0) (< (`KismetMathLibrary.Abs` (- (.y (`self.K2_GetActorLocation`)) _nowtarget_y)) 100.0))
    (set `self.State` "NewEnumerator0")))

(event `カスタムイベント_0`
  (`SkeletalMeshComponent.PlayAnimation` (`self.Mesh`) "/Game/AnimalVarietyPack/Wolf/Animations/ANIM_Wolf_Walk.ANIM_Wolf_Walk" false))

(event `/Game/MyContent/BP/System/BP_Interface.Order Dog`
  (params (Val :type Boolean))
  (`KismetSystemLibrary.PrintText` (`KismetTextLibrary.Conv_BoolToText` Val))
  (`BlackboardComponent.SetValueAsBool` (`AIBlueprintHelperLibrary.GetBlackboard` null) (`self.TargetOderCheckName`) Val))

(event `self.ReceiveTick`
  (params (DeltaSeconds :type "Float (single-precision)"))
  (bind _returnvalue (`AIBlueprintHelperLibrary.GetBlackboard` null))
  (bind _playerdistancename (`self.PlayerDistanceName`))
  (bind _returnvalue_2 (`self.GetDistanceTo` (`GameplayStatics.GetPlayerPawn` 0)))
  ;[1 1 1] Tick
  (`|ExecutionSequence`
    (:`then_0`
      ;;[1 1 1] Playerからもっと近い氷を調べる
      (set `self.MInDistance` 2000000.0)
      (bind _outactors (`GameplayStatics.GetAllActorsOfClass` "/Game/MyContent/BP/Object/BP_TargetDog.BP_TargetDog_C"))
      (for _array_element _outactors
        (if (< _returnvalue_2 (`self.MInDistance`))
          (set `self.MInDistance` _returnvalue_2)
          (set `self.Array Element_2` _array_element)))
      (`BlackboardComponent.SetValueAsObject` (`AIBlueprintHelperLibrary.GetBlackboard` null) (`self.AppleTargetActorCheckName`) (`self.Array Element_2`)))
    (:`then_1`
      ;;[1 1 1] Playerから一定以上離れているか？
      (bind _outactors_2 (`GameplayStatics.GetAllActorsOfClass` "/Game/MyContent/BP/Object/BP_TargetDog.BP_TargetDog_C"))
      (for _array_element_2 _outactors_2
        (bind _returnvalue_3 (`self.GetDistanceTo` (`GameplayStatics.GetPlayerPawn` 0) _array_element_2))
        (`KismetSystemLibrary.PrintText` (`KismetTextLibrary.Conv_DoubleToText` _returnvalue_3 "HalfToEven") true true (struct :`G` 0.66 :`B` 1.0 :`A` 1.0) 0.0)
        (if (>= _returnvalue_3 1500.0)
          (bind _output_get (set `self.NewVar_2` false))
          (`BlackboardComponent.SetValueAsBool` _returnvalue _playerdistancename _output_get)
          (else
            (bind _output_get_2 (set `self.NewVar_2` true))
            (`BlackboardComponent.SetValueAsBool` _returnvalue _playerdistancename _output_get_2)))))))

(fn `Ground Check`
  (bind _mesh (`self.Mesh`))
  (set `self.NoSnow` false)
  (message `/Game/MyContent/BP/System/BP_Interface.Collision Check` (`GameplayStatics.GetGameMode`) (`self.GroundRange`))
  (if true
    (`SceneComponent.K2_SetRelativeLocation` _mesh (0.0 0.0 -90.0) true false)
    (else
      (`SceneComponent.K2_SetRelativeLocation` _mesh (0.0 0.0 -40.0) true false))))

(fn `UserConstructionScript`
  (`/Game/MyContent/TrailSystem/Blueprints/BP_TrailVisualizer.VisualizeTrailComponents`))